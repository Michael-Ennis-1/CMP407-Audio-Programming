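; Player audio component that drives Wwise music and footstep sounds.
; BeginPlay starts the hidden music on the owner, and callable events post Wwise events to switch between chase and hidden music or play footsteps.
; SwitchFootsteps reads the passed actor's tags to set the owner's surface switch for footsteps, printing a colored debug message for each match.
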(event EventBeginPlay
  (Class|AkGameplayStatics|PostEvent "/Game/WwiseAudio/Events/Default_Work_Unit/DynamicMusic/BeginHiddenMusic.BeginHiddenMusic" (Components|GetOwner)))

(event EventTick
  (params (DeltaSeconds :type Float%20%28single-precision%29)))

(event EventPlayFootsteps
  (Class|AkGameplayStatics|PostEvent "/Game/WwiseAudio/Events/Default_Work_Unit/PlayFootsteps.PlayFootsteps" (Components|GetOwner)))

(event EventSwitchFootsteps
  (params (InOtherActor :type Actor%20Object%20Reference))
  (CallFunction|ApplyWwiseFootstepsSwitch InOtherActor))

(event EventPlayChaseMusic
  (Class|AkGameplayStatics|PostEvent "/Game/WwiseAudio/Events/Default_Work_Unit/DynamicMusic/SetChased.SetChased"))

(event EventPlayHiddenMusic
  (Class|AkGameplayStatics|PostEvent "/Game/WwiseAudio/Events/Default_Work_Unit/DynamicMusic/SetHidden.SetHidden"))

(fn ApplyWwiseFootstepsSwitch
  (params (InActor :type Actor%20Object%20Reference))
  (for _array_element (Variables|/Script/Engine.Actor|GetTags InActor)
    (if (== _array_element "Grass")
      (Class|AkGameplayStatics|SetSwitch "/Game/WwiseAudio/Switches/Default_Work_Unit/FootstepsSwitchGroup/FootstepsSwitchGroup-GrassSwitch.FootstepsSwitchGroup-GrassSwitch" (Components|GetOwner))
      (Development|PrintString "Grass" true true "(R=0.000000,G=1.000000,B=0.255520,A=1.000000)")
      (elif (== _array_element "Metal")
        (Class|AkGameplayStatics|SetSwitch "/Game/WwiseAudio/Switches/Default_Work_Unit/FootstepsSwitchGroup/FootstepsSwitchGroup-MetalSwitch.FootstepsSwitchGroup-MetalSwitch" (Components|GetOwner))
        (Development|PrintString "Metal" true true "(R=0.203125,G=0.270833,B=0.270833,A=1.000000)")
        (elif (== _array_element "Water")
          (Class|AkGameplayStatics|SetSwitch "/Game/WwiseAudio/Switches/Default_Work_Unit/FootstepsSwitchGroup/FootstepsSwitchGroup-WaterSwitch.FootstepsSwitchGroup-WaterSwitch" (Components|GetOwner))
          (Development|PrintString "Water" true true "(R=0.000000,G=0.799628,B=1.000000,A=1.000000)"))))))