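; Player character Blueprint that takes damage on contact with audio enemies and can be returned to its starting point.
; A capsule overlap with a BP_AudioEnemy disables that enemy and removes a fixed amount of health through the player's health component.
; BeginPlay caches the starting location and rotation, which RespawnPlayer restores when called.
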(event OnComponentBeginOverlap(CapsuleComponent)
  (params (OverlappedComponent :type Primitive%20Component%20Object%20Reference) (OtherActor :type Actor%20Object%20Reference) (OtherComp :type Primitive%20Component%20Object%20Reference) (OtherBodyIndex :type Integer) (bFromSweep :type Boolean) (SweepResult :type Hit%20Result%20Structure%20%28by%20ref%29))
  (bind _asbp_audio_enemy (Utilities|Casting|CastToBP_AudioEnemy OtherActor))
  (Class|AudioEnemy|DisableEnemy _asbp_audio_enemy)
  (Class|AudioPlayerHealthComponent|RemoveHealth (Variables|Default|GetBP_AudioPlayerHealthComponent) 3e+01))

(event EventBeginPlay
  (Variables|Default|SetPlayerStartingPosition (Transformation|GetActorLocation))
  (Variables|Default|SetPlayerStartingRotation (Transformation|GetActorRotation)))

(event Collision|EventActorBeginOverlap
  (params (OtherActor :type Actor%20Object%20Reference)))

(event EventTick
  (params (DeltaSeconds :type Float%20%28single-precision%29)))

(fn ConstructionScript)

(fn RespawnPlayer
  (Transformation|SetActorLocationAndRotation (Variables|Default|GetPlayerStartingPosition) (Variables|Default|GetPlayerStartingRotation)))