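; Player character Blueprint that drives a Wwise dynamic audio loop from whether the player is moving.
; BeginPlay posts the loop event and initializes the PlayerSpeed RTPC.
; Each tick writes an accumulated float to that RTPC, then ramps it up while velocity exceeds a small threshold or down otherwise.
; The value is clamped and uses separate moving and stationary ramp times, so it reflects movement duration rather than actual speed.
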(event EventBeginPlay
  (Class|AkGameplayStatics|PostEvent "/Game/WwiseAudio/Events/Default_Work_Unit/StartDynamicLoop.StartDynamicLoop")
  (Class|AkGameplayStatics|SetRTPCValue "/Game/WwiseAudio/Game_Parameters/Default_Work_Unit/PlayerSpeed.PlayerSpeed" 0.0))

(event Collision|EventActorBeginOverlap
  (params (OtherActor :type Actor%20Object%20Reference)))

(event EventTick
  (params (DeltaSeconds :type Float%20%28single-precision%29))
  (Class|AkGameplayStatics|SetRTPCValue "/Game/WwiseAudio/Game_Parameters/Default_Work_Unit/PlayerSpeed.PlayerSpeed" (Variables|Default|GetTestFloat))
  (if (> (Math|Vector|VectorLength (Transformation|GetVelocity)) 1.0)
    (Variables|Default|SetTestFloat (Math|Float|Clamp(Float) (+ (Variables|Default|GetTestFloat) (* DeltaSeconds (/ (Variables|Default|GetFullRTPCValue) (Variables|Default|GetMovingSeconds)))) 0.0 1e+02))
    (else
      (Variables|Default|SetTestFloat (Math|Float|Clamp(Float) (- (Variables|Default|GetTestFloat) (* DeltaSeconds (/ (Variables|Default|GetFullRTPCValue) (Variables|Default|GetStationarySeconds)))) 0.0 1e+02)))))

(fn ConstructionScript)