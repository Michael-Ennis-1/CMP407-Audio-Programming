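; BP_EnemyAudioComponent is an enemy component that plays Wwise sound effects for gunfire and explosions.
; Gunshot and explosion events post Ak events on the owning actor.
; The explosion event also disables collision on the meshes, capsule and box collider of an owning BP_AudioEnemy.
; A separate respawn variant posts the explosion at the owner's location, oriented by its AI controller's control rotation.
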(event EventPlayExplosionSFX
  (bind _returnvalue (Components|GetOwner))
  (Class|AkGameplayStatics|PostEvent "/Game/WwiseAudio/Events/Default_Work_Unit/SoundEffects/PlayExplosion.PlayExplosion" _returnvalue)
  (bind _asbp_audio_enemy (Utilities|Casting|CastToBP_AudioEnemy _returnvalue))
  (Collision|SetCollisionEnabled (Variables|/Game/CMP407Content/AI/BP_AudioEnemy.BP_AudioEnemy_C|GetStaticMesh _asbp_audio_enemy) "NoCollision")
  (Collision|SetCollisionEnabled (Variables|/Game/CMP407Content/AI/BP_AudioEnemy.BP_AudioEnemy_C|GetStaticMesh1 _asbp_audio_enemy) "NoCollision")
  (Collision|SetCollisionEnabled (Variables|/Game/CMP407Content/AI/BP_AudioEnemy.BP_AudioEnemy_C|GetStaticMesh2 _asbp_audio_enemy) "NoCollision")
  (Collision|SetCollisionEnabled (Variables|/Script/Engine.Character|GetMesh _asbp_audio_enemy) "NoCollision")
  (Collision|SetCollisionEnabled (Variables|/Script/Engine.Character|GetCapsuleComponent _asbp_audio_enemy) "NoCollision")
  (Collision|SetCollisionEnabled (Variables|/Game/CMP407Content/AI/BP_AudioEnemy.BP_AudioEnemy_C|GetBoxCollider _asbp_audio_enemy) "NoCollision"))

(event EventPlayBulletSFX
  (Class|AkGameplayStatics|PostEvent "/Game/WwiseAudio/Events/Default_Work_Unit/SoundEffects/PlayGunshot.PlayGunshot" (Components|GetOwner)))

(fn PlayExplosionwithRespawn
  (bind _returnvalue (Components|GetOwner))
  (Class|AkGameplayStatics|PostEventatLocation "/Game/WwiseAudio/Events/Default_Work_Unit/SoundEffects/PlayExplosion.PlayExplosion" (Transformation|GetActorLocation _returnvalue) (Pawn|GetControlRotation (AI|GetAIController _returnvalue) :!class /Script/Engine.Controller)))